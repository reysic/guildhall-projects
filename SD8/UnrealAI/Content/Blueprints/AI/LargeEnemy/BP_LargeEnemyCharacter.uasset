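; Large enemy AI character that takes damage, fires projectiles and is destroyed when its health runs out.
; Timestamped damage arrays form a rolling recent-damage total; crossing a threshold, or any hit in the post-flee state, triggers fleeing unless another state blocks it.
; Tick prunes that window and ends fleeing after a damage-free duration, writing state to the Blackboard.
; Optional debug drawing shows ranges, aggro cone, health, state and recent damage.
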(event EventTick
  (params (DeltaSeconds :type Float%20%28single-precision%29))
  (CallFunction|RemovefromDamageArrays)
  (CallFunction|UpdateRecentDamageTaken)
  (CallFunction|CheckifShouldStillbeFleeing)
  (if (Variables|Default|GetDrawDebugIndicators)
    (CallFunction|DrawAggroRangeIndicator)
    (CallFunction|DrawFrontalAggroDegreesIndicator)
    (CallFunction|DrawHealthIndicator)
    (CallFunction|DrawAIStateIndicator)
    (CallFunction|DrawWanderRadiusIndicator)
    (CallFunction|DrawRecentDamageIndicator)
    (CallFunction|DrawStartleRadiusIndicator)))

(event Game|Damage|EventAnyDamage
  (params (Damage :type Float%20%28single-precision%29) (DamageType :type Damage%20Type%20Object%20Reference) (InstigatedBy :type Controller%20Object%20Reference) (DamageCauser :type Actor%20Object%20Reference))
  ;[1 1 1] Take Damage
  (if (CallFunction|IsAlive)
    (bind _output_get (Variables|Default|SetCurrentHealth (Math|Float|Clamp(Float) (- (Variables|Default|GetCurrentHealth) Damage) 0.0 (Variables|Default|GetMaxHealth))))
    (if (== _output_get 0.0)
      (AI|Components|Blackboard|SetValueasEnum (AI|GetBlackboard self) (Utilities|Name|MakeLiteralName "CurrentAIState") (Utilities|Enum|LiteralenumENUM_LargeEnemyAIStates "NewEnumerator4"))
      (CallFunction|Die)
      (else
        (CallFunction|AddtoDamageArrays (Utilities|Time|GetGameTimeinSeconds) Damage)
        (Variables|Default|SetTimeLastDamaged (Utilities|Time|GetGameTimeinSeconds))
        (CallFunction|UpdateRecentDamageTaken)
        (if (and (or (>= (Variables|Default|GetRecentDamageTaken) (Variables|Default|GetRecentDamageThreshold)) (== (Class|BlackboardComponent|GetValueasEnum (AI|GetBlackboard self) (Utilities|Name|MakeLiteralName "CurrentAIState")) (Utilities|Enum|LiteralenumENUM_LargeEnemyAIStates "NewEnumerator6"))) (!= (Class|BlackboardComponent|GetValueasEnum (AI|GetBlackboard self) (Utilities|Name|MakeLiteralName "CurrentAIState")) (Utilities|Enum|LiteralenumENUM_LargeEnemyAIStates "NewEnumerator8")))
          (AI|Components|Blackboard|SetValueasEnum (AI|GetBlackboard self) (Utilities|Name|MakeLiteralName "CurrentAIState") (Utilities|Enum|LiteralenumENUM_LargeEnemyAIStates "NewEnumerator5")))))))

(event EventAttack
  ;[1 1 1] Attack
  (Game|SpawnActorfromClass "/Game/Blueprints/AI/LargeEnemy/BP_LargeEnemyProjectile.BP_LargeEnemyProjectile_C" (Math|Transform|MakeTransform (Transformation|GetWorldLocation (Variables|Default|GetProjectileSpawn)) (Transformation|GetActorRotation)) "AdjustIfPossibleButDontSpawnIfColliding" 0 0))

(event EventDie
  ;[1 1 1] Die
  (Actor|DestroyActor))

(fn ConstructionScript
  (Variables|Default|SetCurrentHealth (Variables|Default|GetMaxHealth))
  (Variables|Default|SetBaseMoveSpeed (Variables|/Script/Engine.CharacterMovementComponent|GetMaxWalkSpeed (Variables|Character|GetCharacterMovement))))

(fn DrawAggroRangeIndicator
  (Rendering|Debug|DrawDebugCircle (Transformation|GetActorLocation) (Variables|Default|GetAggroRange) 500 "(R=1.000000,G=0.000000,B=0.000000,A=1.000000)" 0.0 5.0 "0.000000,1.000000,0.000000" "1.000000,0.000000,0.000000")
  (return))

(fn DrawHealthIndicator
  (Rendering|Components|TextRender|SetText (Variables|Default|GetCurrentHealthText) (Utilities|Text|ToText(String) (Utilities|String|Append (Utilities|String|ToString(Float) (Variables|Default|GetCurrentHealth)) " / " (Utilities|String|ToString(Float) (Variables|Default|GetMaxHealth)))))
  (Rendering|SetVisibility (Variables|Default|GetCurrentHealthText) true false)
  (CallFunction|BillboardTextIndicator (Variables|Default|GetCurrentHealthText))
  (return))

(fn DrawAIStateIndicator
  (bind _returnvalue (AI|GetAIController self))
  (bind _asbp_large_enemy_controller (Utilities|Casting|CastToBP_LargeEnemyController _returnvalue)
    (:then
      (bind _output_get (LocalVariables|SetCurrentAIState (Utilities|Enum|ByteToEnumENUM_SmallEnemyAnimationStates (Class|BlackboardComponent|GetValueasEnum (AI|GetBlackboard _asbp_large_enemy_controller) (Utilities|Name|MakeLiteralName "CurrentAIState")))))
      (Rendering|Components|TextRender|SetText (Variables|Default|GetCurrentAIStateText) (Utilities|Text|ToText(String) (Utilities|String|EnumtoString _output_get)))
      (Rendering|SetVisibility (Variables|Default|GetCurrentAIStateText) true false)
      (CallFunction|BillboardTextIndicator (Variables|Default|GetCurrentAIStateText))
      (return))
    (:CastFailed
      (Development|PrintString "Cast failed to BP_LargeEnemyController in BP_LargeEnemyCharacter")
      (return))))

(fn BillboardTextIndicator
  (params (TextRenderComponent :type Text%20Render%20Component%20Object%20Reference))
  (bind _asfirst_person_character (Utilities|Casting|CastToFirstPersonCharacter (Game|GetPlayerCharacter 0)))
  (Transformation|SetWorldRotation TextRenderComponent (Math|Rotator|FindLookatRotation (Transformation|GetWorldLocation TextRenderComponent) (Transformation|GetWorldLocation (Variables|/Game/FirstPersonBP/Blueprints/FirstPersonCharacter.FirstPersonCharacter_C|GetFirstPersonCamera _asfirst_person_character))) false false))

(fn DrawFrontalAggroDegreesIndicator
  (bind _returnvalue (Transformation|GetActorLocation))
  (bind _returnvalue_2 (Transformation|GetActorRotation))
  (bind _returnvalue_3 (Transformation|GetActorLocation))
  (bind _returnvalue_4 (Transformation|GetActorRotation))
  (bind (_roll _pitch _yaw) (Math|Rotator|BreakRotator _returnvalue_2))
  (bind (_roll_2 _pitch_2 _yaw_2) (Math|Rotator|BreakRotator _returnvalue_4))
  (Rendering|Debug|DrawDebugLine _returnvalue_3 (+ _returnvalue_3 (* (Math|Vector|GetForwardVector (Math|Rotator|MakeRotator _roll_2 _pitch_2 (- _yaw_2 (/ (Variables|Default|GetFrontalAggroDegrees) 2.0)))) (Variables|Default|GetAggroRange))) "(R=1.000000,G=0.000000,B=0.000000,A=1.000000)" 0.0 5.0)
  (Rendering|Debug|DrawDebugLine _returnvalue (+ _returnvalue (* (Math|Vector|GetForwardVector (Math|Rotator|MakeRotator _roll _pitch (+ _yaw (/ (Variables|Default|GetFrontalAggroDegrees) 2.0)))) (Variables|Default|GetAggroRange))) "(R=1.000000,G=0.000000,B=0.000000,A=1.000000)" 0.0 5.0)
  (return))

(fn IsAlive
  (return (> (Variables|Default|GetCurrentHealth) 0.0)))

(fn DrawWanderRadiusIndicator
  (Rendering|Debug|DrawDebugCircle (AI|Components|Blackboard|GetValueasVector (AI|GetBlackboard self) (Utilities|Name|MakeLiteralName "HomeLocation")) (Variables|Default|GetWanderRadius) 500 "(R=0.000000,G=1.000000,B=1.000000,A=1.000000)" 0.0 5.0 "0.000000,1.000000,0.000000" "1.000000,0.000000,0.000000")
  (return))

(fn DrawRecentDamageIndicator
  (Rendering|Components|TextRender|SetText (Variables|Default|GetRecentDamageText) (Utilities|Text|ToText(Float) (Variables|Default|GetRecentDamageTaken) "HalfToEven"))
  (Rendering|SetVisibility (Variables|Default|GetRecentDamageText) true false)
  (CallFunction|BillboardTextIndicator (Variables|Default|GetRecentDamageText))
  (return))

(fn AddtoDamageArrays
  (params (DamageTime :type Float%20%28single-precision%29) (DamageAmount :type Float%20%28single-precision%29))
  (Utilities|Array|Add (Variables|Default|GetDamageTimes) DamageTime)
  (Utilities|Array|Add (Variables|Default|GetDamageAmounts) DamageAmount)
  (return))

(fn RemovefromDamageArrays
  (bind (_array_element _array_index) (Utilities|Array|ForEachLoopwithBreak (Variables|Default|GetDamageTimes) :!label _label)
    (:LoopBody
      (if (< _array_element (- (Utilities|Time|GetGameTimeinSeconds) (Variables|Default|GetRecentDamageSeconds)))
        (Utilities|Array|RemoveIndex (Variables|Default|GetDamageTimes) _array_index)
        (Utilities|Array|RemoveIndex (Variables|Default|GetDamageAmounts) _array_index)
        (else
          (goto _label Break))))))

(fn UpdateRecentDamageTaken
  (Variables|Default|SetRecentDamageTaken 0.0)
  (for _array_element (Variables|Default|GetDamageAmounts)
    (Variables|Default|SetRecentDamageTaken (+ _array_element (Variables|Default|GetRecentDamageTaken)))))

(fn CheckifShouldStillbeFleeing
  (if (== (Class|BlackboardComponent|GetValueasEnum (AI|GetBlackboard self) (Utilities|Name|MakeLiteralName "CurrentAIState")) (Utilities|Enum|LiteralenumENUM_LargeEnemyAIStates "NewEnumerator5"))
    (if (< (+ (Variables|Default|GetTimeLastDamaged) (Variables|Default|GetFleeDuration)) (Utilities|Time|GetGameTimeinSeconds))
      (AI|Components|Blackboard|SetValueasEnum (AI|GetBlackboard self) (Utilities|Name|MakeLiteralName "CurrentAIState") (Utilities|Enum|LiteralenumENUM_LargeEnemyAIStates "NewEnumerator6")))))

(fn DrawStartleRadiusIndicator
  (Rendering|Debug|DrawDebugCircle (Transformation|GetActorLocation) (Variables|Default|GetStartleRadius) 500 "(R=1.000000,G=1.000000,B=0.000000,A=1.000000)" 0.0 5.0 "0.000000,1.000000,0.000000" "1.000000,0.000000,0.000000")
  (return))