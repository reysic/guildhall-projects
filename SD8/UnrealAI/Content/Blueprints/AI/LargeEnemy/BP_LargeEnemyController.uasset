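; AI controller for the large enemy character that starts its behavior tree when it possesses the pawn.
; On possess it casts to BP_LargeEnemyCharacter, initializes BB_LargeEnemy and records the pawn's spawn position as HomeLocation.
; It copies the character's aggro, movement, wander, flee, alert and startle tuning into the blackboard, so per-character settings drive BT_LargeEnemy.
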(event EventOnPossess
  (params (PossessedPawn :type Pawn%20Object%20Reference))
  (bind _self self)
  (bind _returnvalue (AI|GetBlackboard _self))
  (bind _asbp_large_enemy_character (Utilities|Casting|CastToBP_LargeEnemyCharacter PossessedPawn))
  (Variables|Default|SetEnemyCharacterRef _asbp_large_enemy_character)
  (Class|AIController|UseBlackboard "/Game/Blueprints/AI/LargeEnemy/BB_LargeEnemy.BB_LargeEnemy")
  (AI|Components|Blackboard|SetValueasVector _returnvalue (Utilities|Name|MakeLiteralName "HomeLocation") (Transformation|GetActorLocation (Pawn|GetControlledPawn)))
  (AI|Components|Blackboard|SetValueasFloat _returnvalue (Utilities|Name|MakeLiteralName "AggroRange") (Variables|/Game/Blueprints/AI/LargeEnemy/BP_LargeEnemyCharacter.BP_LargeEnemyCharacter_C|GetAggroRange (Variables|Default|GetEnemyCharacterRef)))
  (AI|Components|Blackboard|SetValueasFloat _returnvalue (Utilities|Name|MakeLiteralName "FrontalAggroDegrees") (Variables|/Game/Blueprints/AI/LargeEnemy/BP_LargeEnemyCharacter.BP_LargeEnemyCharacter_C|GetFrontalAggroDegrees (Variables|Default|GetEnemyCharacterRef)))
  (AI|Components|Blackboard|SetValueasFloat _returnvalue (Utilities|Name|MakeLiteralName "BaseMoveSpeed") (Variables|/Game/Blueprints/AI/LargeEnemy/BP_LargeEnemyCharacter.BP_LargeEnemyCharacter_C|GetBaseMoveSpeed (Variables|Default|GetEnemyCharacterRef)))
  (AI|Components|Blackboard|SetValueasFloat _returnvalue (Utilities|Name|MakeLiteralName "WanderSpeed") (Variables|/Game/Blueprints/AI/LargeEnemy/BP_LargeEnemyCharacter.BP_LargeEnemyCharacter_C|GetWanderSpeed (Variables|Default|GetEnemyCharacterRef)))
  (AI|Components|Blackboard|SetValueasFloat _returnvalue (Utilities|Name|MakeLiteralName "WanderRadius") (Variables|/Game/Blueprints/AI/LargeEnemy/BP_LargeEnemyCharacter.BP_LargeEnemyCharacter_C|GetWanderRadius (Variables|Default|GetEnemyCharacterRef)))
  (AI|Components|Blackboard|SetValueasFloat _returnvalue (Utilities|Name|MakeLiteralName "AggressiveMoveSpeed") (Variables|/Game/Blueprints/AI/LargeEnemy/BP_LargeEnemyCharacter.BP_LargeEnemyCharacter_C|GetAggressiveMoveSpeed (Variables|Default|GetEnemyCharacterRef)))
  (AI|Components|Blackboard|SetValueasFloat _returnvalue (Utilities|Name|MakeLiteralName "WanderingChance") (Variables|/Game/Blueprints/AI/LargeEnemy/BP_LargeEnemyCharacter.BP_LargeEnemyCharacter_C|GetWanderingChance (Variables|Default|GetEnemyCharacterRef)))
  (AI|Components|Blackboard|SetValueasFloat _returnvalue (Utilities|Name|MakeLiteralName "FleeSpeed") (Variables|/Game/Blueprints/AI/LargeEnemy/BP_LargeEnemyCharacter.BP_LargeEnemyCharacter_C|GetFleeSpeed (Variables|Default|GetEnemyCharacterRef)))
  (AI|Components|Blackboard|SetValueasFloat _returnvalue (Utilities|Name|MakeLiteralName "FleeRadius") (Variables|/Game/Blueprints/AI/LargeEnemy/BP_LargeEnemyCharacter.BP_LargeEnemyCharacter_C|GetFleeRadius (Variables|Default|GetEnemyCharacterRef)))
  (AI|Components|Blackboard|SetValueasFloat _returnvalue (Utilities|Name|MakeLiteralName "DamageAlertDuration") (Variables|/Game/Blueprints/AI/LargeEnemy/BP_LargeEnemyCharacter.BP_LargeEnemyCharacter_C|GetDamageAlertDuration (Variables|Default|GetEnemyCharacterRef)))
  (AI|Components|Blackboard|SetValueasFloat _returnvalue (Utilities|Name|MakeLiteralName "StartleRadius") (Variables|/Game/Blueprints/AI/LargeEnemy/BP_LargeEnemyCharacter.BP_LargeEnemyCharacter_C|GetStartleRadius (Variables|Default|GetEnemyCharacterRef)))
  (AI|RunBehaviorTree "/Game/Blueprints/AI/LargeEnemy/BT_LargeEnemy.BT_LargeEnemy"))

(fn ConstructionScript)