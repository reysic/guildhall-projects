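; AI controller for small enemies that starts their behavior tree when it possesses a BP_SmallEnemyCharacter.
; On possess it loads BB_SmallEnemy and records the pawn's spawn-time position as HomeLocation.
; It copies the character's tuning values for aggro, movement, wandering, fleeing, damage alert and startle into blackboard keys, then runs BT_SmallEnemy, so tuning lives on the character.
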(event EventOnPossess
  (params (PossessedPawn :type Pawn%20Object%20Reference))
  (bind _self self)
  (bind _returnvalue (AI|GetBlackboard _self))
  (bind _asbp_small_enemy_character (Utilities|Casting|CastToBP_SmallEnemyCharacter PossessedPawn))
  (Variables|Default|SetEnemyCharacterRef _asbp_small_enemy_character)
  (Class|AIController|UseBlackboard "/Game/Blueprints/AI/SmallEnemy/BB_SmallEnemy.BB_SmallEnemy")
  (AI|Components|Blackboard|SetValueasVector _returnvalue (Utilities|Name|MakeLiteralName "HomeLocation") (Transformation|GetActorLocation (Pawn|GetControlledPawn)))
  (AI|Components|Blackboard|SetValueasFloat _returnvalue (Utilities|Name|MakeLiteralName "AggroRange") (Variables|/Game/Blueprints/AI/SmallEnemy/BP_SmallEnemyCharacter.BP_SmallEnemyCharacter_C|GetAggroRange (Variables|Default|GetEnemyCharacterRef)))
  (AI|Components|Blackboard|SetValueasFloat _returnvalue (Utilities|Name|MakeLiteralName "FrontalAggroDegrees") (Variables|/Game/Blueprints/AI/SmallEnemy/BP_SmallEnemyCharacter.BP_SmallEnemyCharacter_C|GetFrontalAggroDegrees (Variables|Default|GetEnemyCharacterRef)))
  (AI|Components|Blackboard|SetValueasFloat _returnvalue (Utilities|Name|MakeLiteralName "BaseMoveSpeed") (Variables|/Game/Blueprints/AI/SmallEnemy/BP_SmallEnemyCharacter.BP_SmallEnemyCharacter_C|GetBaseMoveSpeed (Variables|Default|GetEnemyCharacterRef)))
  (AI|Components|Blackboard|SetValueasFloat _returnvalue (Utilities|Name|MakeLiteralName "WanderSpeed") (Variables|/Game/Blueprints/AI/SmallEnemy/BP_SmallEnemyCharacter.BP_SmallEnemyCharacter_C|GetWanderSpeed (Variables|Default|GetEnemyCharacterRef)))
  (AI|Components|Blackboard|SetValueasFloat _returnvalue (Utilities|Name|MakeLiteralName "WanderRadius") (Variables|/Game/Blueprints/AI/SmallEnemy/BP_SmallEnemyCharacter.BP_SmallEnemyCharacter_C|GetWanderRadius (Variables|Default|GetEnemyCharacterRef)))
  (AI|Components|Blackboard|SetValueasFloat _returnvalue (Utilities|Name|MakeLiteralName "AggressiveMoveSpeed") (Variables|/Game/Blueprints/AI/SmallEnemy/BP_SmallEnemyCharacter.BP_SmallEnemyCharacter_C|GetAggressiveMoveSpeed (Variables|Default|GetEnemyCharacterRef)))
  (AI|Components|Blackboard|SetValueasFloat _returnvalue (Utilities|Name|MakeLiteralName "WanderingChance") (Variables|/Game/Blueprints/AI/SmallEnemy/BP_SmallEnemyCharacter.BP_SmallEnemyCharacter_C|GetWanderingChance (Variables|Default|GetEnemyCharacterRef)))
  (AI|Components|Blackboard|SetValueasFloat _returnvalue (Utilities|Name|MakeLiteralName "FleeSpeed") (Variables|/Game/Blueprints/AI/SmallEnemy/BP_SmallEnemyCharacter.BP_SmallEnemyCharacter_C|GetFleeSpeed (Variables|Default|GetEnemyCharacterRef)))
  (AI|Components|Blackboard|SetValueasFloat _returnvalue (Utilities|Name|MakeLiteralName "FleeRadius") (Variables|/Game/Blueprints/AI/SmallEnemy/BP_SmallEnemyCharacter.BP_SmallEnemyCharacter_C|GetFleeRadius (Variables|Default|GetEnemyCharacterRef)))
  (AI|Components|Blackboard|SetValueasFloat _returnvalue (Utilities|Name|MakeLiteralName "DamageAlertDuration") (Variables|/Game/Blueprints/AI/SmallEnemy/BP_SmallEnemyCharacter.BP_SmallEnemyCharacter_C|GetDamageAlertDuration (Variables|Default|GetEnemyCharacterRef)))
  (AI|Components|Blackboard|SetValueasFloat _returnvalue (Utilities|Name|MakeLiteralName "StartleRadius") (Variables|/Game/Blueprints/AI/SmallEnemy/BP_SmallEnemyCharacter.BP_SmallEnemyCharacter_C|GetStartleRadius (Variables|Default|GetEnemyCharacterRef)))
  (AI|RunBehaviorTree "/Game/Blueprints/AI/SmallEnemy/BT_SmallEnemy.BT_SmallEnemy"))

(fn ConstructionScript)